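; Till actor, apparently for an ordering area, that carries a tutorial indicator and a background widget component.
; The changelocoftut event alternates on each call between showing the indicator at Loc2 and hiding it at Loc1, using a FlipFlop.
; Disconnected logic would enlarge the background widget's draw size on hover, but it never runs.
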(event Custom|changelocoftut
  (bind _tutind (Variables|Default|GetTUTind))
  (bind _tutind_2 (Variables|Default|GetTUTind))
  (Utilities|FlowControl|FlipFlop
    (:A
      (Transformation|SetWorldLocation _tutind (Transformation|GetWorldLocation (Variables|Default|Getloc2)) false false)
      (Rendering|SetVisibility _tutind_2 true false))
    (:B
      (Transformation|SetWorldLocation _tutind (Transformation|GetWorldLocation (Variables|Default|Getloc1)) false false)
      (Rendering|SetVisibility _tutind_2 false false))))

(event EventBeginPlay)

(event Collision|EventActorBeginOverlap
  (params (OtherActor :type Actor%20Object%20Reference)))

(event EventTick
  (params (DeltaSeconds :type Float%20%28single-precision%29)))

(fn ConstructionScript)