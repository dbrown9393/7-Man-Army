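; Customer NPC for a coffee-serving game that orders a random drink, waits on a timer and accepts a matching cup.
; SelectRandomCoffeeOrder picks from one of two coffee-type lists and shows the paired order widget.
; HappinessLevel maps remaining TimeBar time to mood widgets, spawning a fail UI on timeout.
; ReceiveOrder destroys a correct cup and hides order and timer widgets, while QueueTargetAvailable frees the NPC's queue slot.
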(event EventBeginPlay
  (Utilities|FlowControl|Sequence
    (:then_0
      (bind _astime_bar (Utilities|Casting|CastToTimeBar (UserInterface|GetUserWidgetObject (Variables|Default|GetWidgetTimer))))
      (Variables|Default|SetTimeBarRef _astime_bar))))

(fn ConstructionScript)

(fn SelectRandomCoffeeOrder
  (bind _output_get (Variables|Default|SetCoffeeOrder (Utilities|Enum|ByteToEnumCoffeeType_Enum (Math|Conversions|ToByte(Integer) (Math|Random|RandomInteger 6)))))
  (if (Math|Boolean|ORBoolean (Utilities|Enum|Equal(Enum) _output_get "NewEnumerator0") (Utilities|Enum|Equal(Enum) _output_get "NewEnumerator2") (Utilities|Enum|Equal(Enum) _output_get "NewEnumerator3"))
    (Variables|Default|SetOrderDecision true)
    (bind _output_get_2 (Variables|Default|SetOrder%20Number (Utilities|Array|FindItem (Variables|Default|GetCoffeeOrderType) _output_get)))
    (bind _returnvalue (UserInterface|CreateWidget (Utilities|Array|Get(acopy) (Variables|Default|GetOrderWifget) _output_get_2)))
    (UserInterface|SetWidget (Variables|Default|GetWidget) _returnvalue)
    (else
      (Variables|Default|SetOrderDecision false)
      (bind _output_get_3 (Variables|Default|SetOrder%20Number (Utilities|Array|FindItem (Variables|Default|GetOtherCoffeeTypes) _output_get)))
      (bind _returnvalue_2 (UserInterface|CreateWidget (Utilities|Array|Get(acopy) (Variables|Default|GetOtherOrderWifget) _output_get_3)))
      (UserInterface|SetWidget (Variables|Default|GetWidget) _returnvalue_2))))

(fn QueueTargetAvailable
  (bind _queueindex (Variables|Default|GetQueueIndex))
  (bind _returnvalue (Actor|GetActorOfClass (Variables|Default|GetQueues)))
  (bind _structout (Utilities|Struct|Setmembersinqueue_Struct (Utilities|Array|Get(acopy) (Variables|/Game/AI/NPC/Queue.Queue_C|Getqueue%20targets _returnvalue) _queueindex) false))
  (Utilities|Array|SetArrayElem (Variables|/Game/AI/NPC/Queue.Queue_C|Getqueue%20targets _returnvalue) _queueindex _structout))

(fn HappinessLevel
  (bind _timebarref (Variables|Default|GetTimeBarRef))
  (bind _time (Variables|/Game/AI/NPC/TimeBar.TimeBar_C|GetTime _timebarref))
  (Utilities|IsValid _timebarref
    (:Is%20Valid
      (if (> _time 0.4)
        (bind _returnvalue (UserInterface|CreateWidget "/Game/AI/UI/Happy_WB.Happy_WB_C"))
        (UserInterface|SetWidget (Variables|Default|GetHappiness) _returnvalue)
        (elif (and (< _time 0.4) (> _time 0.2))
          (bind _returnvalue_2 (UserInterface|CreateWidget "/Game/AI/UI/Content_WB.Content_WB_C"))
          (UserInterface|SetWidget (Variables|Default|GetHappiness) _returnvalue_2)
          (elif (and (< _time 0.2) (> _time 0.0))
            (bind _returnvalue_3 (UserInterface|CreateWidget "/Game/AI/UI/Angry_WB.Angry_WB_C"))
            (UserInterface|SetWidget (Variables|Default|GetHappiness) _returnvalue_3)
            (elif (and (!= (Variables|Default|GetOrderReceived?) true) (<= _time 0.0))
              (Game|SpawnActorfromClass "/Game/dylan_UI/customer/failUI_BP1.failUI_BP1_C" (Math|Transform|MakeTransform (Transformation|GetWorldLocation (Variables|Default|GetScene)) "0, 0, 0" "1.000000,1.000000,1.000000") "Undefined" 0 0))))))))

(fn ReceiveOrder
  (params (Cup :type Actor%20Object%20Reference) (Coffee%20Type :type CoffeeType_Enum%20Enum :default "NewEnumerator0"))
  (bind _order_number (Variables|Default|GetOrder%20Number))
  (Utilities|IsValid Cup
    (:Is%20Valid
      (if (Variables|Default|GetOrderDecision)
        (if (Utilities|Enum|Equal(Enum) (Utilities|Array|Get(acopy) (Variables|Default|GetCoffeeOrderType) _order_number) Coffee%20Type)
          (Actor|DestroyActor Cup :!label _label)
          (Rendering|SetVisibility (Variables|Default|GetWidget) false false)
          (Rendering|SetVisibility (Variables|Default|GetWidgetTimer) false false)
          (Variables|Default|SetOrderReceived? true))
        (elif (Utilities|Enum|Equal(Enum) (Utilities|Array|Get(acopy) (Variables|Default|GetOtherCoffeeTypes) _order_number) Coffee%20Type)
          (goto _label))))))