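; Grabbable VR tamper prop that, while held, tamps a portafilter containing untamped grounds on overlap, setting its Tampered flag and playing a sound.
; Grab and drop events toggle Hold, play sounds and toggle the info widget.
; In tutorial mode, Tick polls hover widgets to drive a custom-depth outline, material swap and one-shot raised info widget.
; A fast looping timer shows a guide arrow while the player's OverTamper flag is set, which grabbing clears.
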(event OnComponentBeginOverlap(Box)
  (params (OverlappedComponent :type Primitive%20Component%20Object%20Reference) (OtherActor :type Actor%20Object%20Reference) (OtherComp :type Primitive%20Component%20Object%20Reference) (OtherBodyIndex :type Integer) (bFromSweep :type Boolean) (SweepResult :type Hit%20Result%20Structure%20%28by%20ref%29))
  (Utilities|FlowControl|Sequence
    (:then_0
      (if (Variables|Default|Gethold)
        (bind _asbp_portafilter (Utilities|Casting|CastToBP_Portafilter OtherActor))
        (if (and (!= (Variables|/Game/Props/Portafilter/BP_Portafilter.BP_Portafilter_C|GetTampered? _asbp_portafilter) true) (== (Variables|/Game/Props/Portafilter/BP_Portafilter.BP_Portafilter_C|GetHasGrounds? _asbp_portafilter) true))
          (Variables|/Game/Props/Portafilter/BP_Portafilter.BP_Portafilter_C|SetTampered? _asbp_portafilter true)
          (Audio|PlaySoundatLocation "/Game/Audio/coffegrounds/tampernoise.tampernoise" (Transformation|GetWorldLocation (Variables|/Game/Props/Portafilter/BP_Portafilter.BP_Portafilter_C|GetSphere _asbp_portafilter)) "0, 0, 0" 1.0 1.0 0.0 0 0 0 0))))))

(event OnDropped(GrabComponent)
  (Audio|PlaySoundatLocation "/Game/Audio/dropobject.dropobject" (Transformation|GetActorLocation self) "0, 0, 0" 1.0 1.0 0.0 0 0 0 0)
  (Variables|Default|Sethold false)
  (Rendering|SetVisibility (Variables|Default|GetmlkjugUI) true false))

(event OnGrabbed(GrabComponent)
  (bind _tamper (Variables|Default|Gettamper))
  (Utilities|FlowControl|Sequence
    (:then_0
      (Audio|PlaySoundatLocation "/Game/Audio/pickupobject.pickupobject" (Transformation|GetActorLocation self) "0, 0, 0" 1.0 1.0 0.0 0 0 0 0)
      (Variables|Default|Sethold true)
      (Rendering|SetRenderCustomDepth _tamper false)
      (Rendering|Material|SetMaterial _tamper 0 "/Game/Props/AutoTamper/the_coffeema.the_coffeema")
      (Rendering|SetVisibility (Variables|Default|GetmlkjugUI) false false))
    (:then_1
      (bind _asvrplayer (Utilities|Casting|CastToVRPlayer (Game|Player|GetPlayerPawn 0)))
      (Variables|/Game/VRTemplate/Blueprints/VRPlayer.VRPlayer_C|SetOverTamper _asvrplayer false))))

(event Custom|outline
  (bind _tamper (Variables|Default|Gettamper))
  (bind _asvrplayer (Utilities|Casting|CastToVRPlayer (Game|Player|GetPlayerPawn 0)))
  (if (Variables|/Game/VRTemplate/Blueprints/VRPlayer.VRPlayer_C|GetTutorial _asvrplayer)
    (if (Math|Boolean|ORBoolean (Widget|IsHovered (UserInterface|GetWidget (Variables|Default|GetWidget4Hover))) (Widget|IsHovered (UserInterface|GetWidget (Variables|Default|Getw1))) (Widget|IsHovered (UserInterface|GetWidget (Variables|Default|Getw2))) (Widget|IsHovered (UserInterface|GetWidget (Variables|Default|GetWidget4Hover2))))
      (if (!= (Variables|Default|Gethold) true)
        (Rendering|SetVisibility (Variables|Default|GetmlkjugUI) true false)
        (Rendering|SetRenderCustomDepth _tamper true)
        (Rendering|Material|SetMaterial _tamper 0 "/Game/Props/CoffeeFrotherJug/theochover.theochover")
        (Utilities|FlowControl|DoOnce false :!label _label
          (:Completed
            (CallFunction|Changeui)
            (Audio|PlaySoundatLocation "/Game/myUI/Sounds/maximize_008.maximize_008" (Variables|/Script/Engine.SceneComponent|GetRelativeLocation (Variables|Default|Gettamper)) "0, 0, 0" 1.0 1.0 0.0 0 0 0 0)))
        (else
          (Rendering|SetVisibility (Variables|Default|GetmlkjugUI) false false)
          (Rendering|SetRenderCustomDepth _tamper false :!label _label_2)
          (Rendering|Material|SetMaterial _tamper 0 "/Game/Props/AutoTamper/the_coffeema.the_coffeema")
          (CallFunction|Changelocback)
          (goto _label Reset)))
      (else
        (goto _label_2)))
    (else
      (Rendering|SetVisibility (Variables|Default|GetmlkjugUI) false false)
      (Rendering|SetVisibility (Variables|Default|GetmlkjugUI) false false)
      (goto _label_2))))

(event Custom|changelocback
  (Transformation|SetRelativeLocation (Variables|Default|GetmlkjugUI) (Variables|/Script/Engine.SceneComponent|GetRelativeLocation (Variables|Default|GetScene)) false false))

(event Custom|changeui
  (bind _mlkjugui (Variables|Default|GetmlkjugUI))
  (bind _returnvalue (Transformation|GetRelativeTransform _mlkjugui))
  (Components|MoveComponentTo _mlkjugui (Math|Vector|MakeVector (.x (.location _returnvalue)) (.y (.location _returnvalue)) (+ (.z (.location _returnvalue)) 2.5)) (.rotation _returnvalue) false false 0.2 false))

(event Custom|realchang)

(event Custom|uopdateloc)

(event Custom|makearrow
  (bind _arrow (Variables|Default|Getarrow))
  (bind _asvrplayer (Utilities|Casting|CastToVRPlayer (Game|Player|GetPlayerPawn 0)))
  (if (and (Variables|/Game/VRTemplate/Blueprints/VRPlayer.VRPlayer_C|GetTutorial _asvrplayer) (Variables|/Game/VRTemplate/Blueprints/VRPlayer.VRPlayer_C|GetOverTamper _asvrplayer))
    (Rendering|SetVisibility _arrow true false)
    (else
      (Rendering|SetVisibility _arrow false false))))

(event EventBeginPlay
  (Utilities|FlowControl|Sequence
    (:then_0
      (Utilities|Time|SetTimerbyEvent (delegate Custom|makearrow) 0.01 true))
    (:then_1
      (Variables|Default|Setdefaultvect (Transformation|GetWorldLocation (Variables|Default|GetmlkjugUI))))))

(event Collision|EventActorBeginOverlap
  (params (OtherActor :type Actor%20Object%20Reference)))

(event EventTick
  (params (DeltaSeconds :type Float%20%28single-precision%29))
  (CallFunction|Outline))

(fn ConstructionScript)