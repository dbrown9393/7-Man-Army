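; Cash register prop that plays a scoring sequence with register and coin sounds.
; The cashscore event starts the Playergiveorderseq sequence through its sequence player.
; Two Sequencer event endpoints on the Blueprint play the cash register and coin sounds at the actor's root location, leaving their timing to the sequence.
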(event Custom|cashscore
  (Sequencer|Player|Play (Variables|/Script/ActorSequence.ActorSequenceComponent|GetSequencePlayer (Variables|Default|Getplayergiveorderseq)) :!class /Script/MovieScene.MovieSceneSequencePlayer))

(event EventBeginPlay)

(event Collision|EventActorBeginOverlap
  (params (OtherActor :type Actor%20Object%20Reference)))

(event EventTick
  (params (DeltaSeconds :type Float%20%28single-precision%29)))

(event Custom|SequenceEvent_0
  (Audio|PlaySoundatLocation "/Game/Audio/cashregist/cashregistersound.cashregistersound" (Transformation|GetWorldLocation (Variables|Default|GetDefaultSceneRoot)) "0, 0, 0" 1.0 1.0 0.0 0 0 0 0))

(event Custom|SequenceEvent_1
  (Audio|PlaySoundatLocation "/Game/Audio/cashregist/coins.coins" (Transformation|GetWorldLocation (Variables|Default|GetDefaultSceneRoot)) "0, 0, 0" 1.0 1.0 0.0 0 0 0 0))

(fn ConstructionScript)