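; Child cup Blueprint for a grabbable VR cup that adds hover feedback and a text widget for the player's tutorial mode.
; Tick passes the cup to its cuphover1 widget and polls five widget components for hover, toggling custom-depth outline, highlight material and a one-shot sound unless held.
; A looping timer turns the text widget toward the player, and an outline event shows it only during the tutorial.
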(event OnGrabbed(GrabComponent)
  (Variables|Default|Setisgrabbed true)
  (Rendering|SetRenderCustomDepth (Variables|Default|GetStaticMesh) false))

(event OnDropped(GrabComponent)
  (Variables|Default|Setisgrabbed false))

(event Custom|outline
  (bind _asvrplayer (Utilities|Casting|CastToVRPlayer (Game|Player|GetPlayerPawn 0)))
  (if (Variables|/Game/VRTemplate/Blueprints/VRPlayer.VRPlayer_C|GetTutorial _asvrplayer)
    (Rendering|SetVisibility (Variables|Default|GetWidget4Text) true false)
    (else
      (Rendering|SetVisibility (Variables|Default|GetWidget4Text) false false))))

(event Custom|ff
  (bind _staticmesh (Variables|Default|GetStaticMesh))
  (bind _staticmesh_2 (Variables|Default|GetStaticMesh))
  (bind _asvrplayer (Utilities|Casting|CastToVRPlayer (Game|Player|GetPlayerPawn 0)))
  (if (and (Variables|/Game/VRTemplate/Blueprints/VRPlayer.VRPlayer_C|GetTutorial _asvrplayer) (Math|Boolean|ORBoolean (Widget|IsHovered (UserInterface|GetWidget (Variables|Default|Getw1))) (Widget|IsHovered (UserInterface|GetWidget (Variables|Default|GetWidget4Hover))) (Widget|IsHovered (UserInterface|GetWidget (Variables|Default|GetWidget4Hover2))) (Widget|IsHovered (UserInterface|GetWidget (Variables|Default|Getw))) (Widget|IsHovered (UserInterface|GetWidget (Variables|Default|GetWidget4Text)))))
    (if (!= (Variables|Default|Getisgrabbed) true)
      (Rendering|SetRenderCustomDepth _staticmesh_2 true)
      (Rendering|Material|SetMaterial _staticmesh 0 "/Game/Props/bluecup_HOVER.bluecup_HOVER")
      (Utilities|FlowControl|DoOnce false :!label _label
        (:Completed
          (Audio|PlaySoundatLocation "/Game/myUI/Sounds/maximize_008.maximize_008" (Variables|/Script/Engine.SceneComponent|GetRelativeLocation (Variables|Default|GetStaticMesh)) "0, 0, 0" 1.0 1.0 0.0 0 0 0 0)))
      (else
        (Rendering|SetRenderCustomDepth _staticmesh_2 false :!label _label_2)
        (Rendering|Material|SetMaterial _staticmesh 0 "/Game/Props/bluecup1.bluecup1")
        (goto _label Reset)))
    (else
      (goto _label_2))))

(event Custom|rotatetext
  (bind _widget4text (Variables|Default|GetWidget4Text))
  (bind _asvrplayer (Utilities|Casting|CastToVRPlayer (Game|Player|GetPlayerPawn 0)))
  (Transformation|SetWorldRotation _widget4text (Math|Rotator|MakeRotator 0.0 (.pitch (Math|Rotator|FindLookatRotation (Transformation|GetActorLocation _asvrplayer) (Transformation|GetWorldLocation _widget4text))) (- (.yaw (Math|Rotator|FindLookatRotation (Transformation|GetActorLocation _asvrplayer) (Transformation|GetWorldLocation _widget4text))) 1.8e+02)) false false))

(event EventBeginPlay
  (|CallParentFunction)
  (Utilities|FlowControl|Sequence
    (:then_1
      (Utilities|Time|SetTimerbyEvent (delegate Custom|rotatetext) 0.01 true))))

(event Collision|EventActorBeginOverlap
  (params (OtherActor :type Actor%20Object%20Reference))
  (|CallParentFunction OtherActor) ; This node is disabled and will not be called.\nDrag off pins to build functionality.
)

(event EventTick
  (params (DeltaSeconds :type Float%20%28single-precision%29))
  (|CallParentFunction DeltaSeconds)
  (Utilities|FlowControl|Sequence
    (:then_0
      (bind _ascuphover_1 (Utilities|Casting|CastTocuphover1 (UserInterface|GetUserWidgetObject (Variables|Default|GetWidget4Text))))
      (Variables|/Game/myUI/Tools/coffeepot/cuphover1.cuphover1_C|SetCupReference _ascuphover_1 self))
    (:then_1
      (CallFunction|Ff))))

(fn ConstructionScript
  (|CallParentFunction))