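; BP_Cup is a grabbable coffee cup prop that tracks its espresso, water and milk, and plays a sound when picked up.
; A looping timer totals the ingredients into the fill amount through a coffee-only macro and prints debug text.
; Tick refreshes type and fill labels, flags the drink once espresso is present, and toggles the liquid indicator.
; DetermineDrinkType holds provisional ratio-based classification, but its timer is disconnected, as is the indicator scaling in the event graph.
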(event OnGrabbed(GrabComponent)
  (Audio|PlaySoundatLocation "/Game/Audio/pickupcup.pickupcup" (Transformation|GetActorLocation self) "0, 0, 0" 1.0 1.0 0.0 0 0 0 0))

(event Custom|CupFillUpdate
  (Utilities|MOnlyifIsCoffee?)
  (Rendering|SetVisibility (Variables|Default|GetLiquidFilledIndicatorModel_Temp) true false)
  (bind _output_get (Variables|Default|SetCupFilledAmount (+ (Variables|Default|GetAmountEspresso) (Variables|Default|GetAmountWater) (Variables|Default|GetAmountMilk))))
  (Development|PrintString (Utilities|String|Append "Dingus" (Utilities|String|ToString(Integer) (Math|Random|RandomIntegerinRange 1 2))) true true "(R=0.000000,G=0.660000,B=1.000000,A=1.000000)" 1.0))

(event Custom|DetermineDrinkType
  (if (Math|Boolean|ORBoolean (Utilities|Enum|Equal(Enum) (Variables|Default|GetCoffeeType) "NewEnumerator0") (Utilities|Enum|Equal(Enum) (Variables|Default|GetCoffeeType) "NewEnumerator2") (Utilities|Enum|Equal(Enum) (Variables|Default|GetCoffeeType) "NewEnumerator3") (Utilities|Enum|Equal(Enum) (Variables|Default|GetCoffeeType) "NewEnumerator6") (Utilities|Enum|Equal(Enum) (Variables|Default|GetCoffeeType) "NewEnumerator7"))
    ;[1 1 1] Coffee Type determinations will change later
    (if (== (Variables|Default|GetAmountEspresso) (Variables|Default|GetCupFilledAmount))
      (Variables|Default|SetCoffeeType "NewEnumerator0")
      (Rendering|SetVisibility (Variables|Default|GetLiquidFilledIndicatorModel_Temp) true false)
      (elif (>= (Variables|Default|GetAmountWater) (Variables|Default|GetAmountEspresso))
        (Variables|Default|SetCoffeeType "NewEnumerator6")
        (elif (== (+ (Variables|Default|GetAmountEspresso) (Variables|Default|GetAmountMilk) 0) (Variables|Default|GetCupFilledAmount))
          (Variables|Default|SetCoffeeType "NewEnumerator0")
          (elif (<= (Variables|Default|GetAmountMilk) (+ (Variables|Default|GetAmountEspresso) 5))
            (Variables|Default|SetCoffeeType "NewEnumerator2")
            (elif (>= (Variables|Default|GetAmountMilk) (+ (Variables|Default|GetAmountEspresso) 5))
              (Variables|Default|SetCoffeeType "NewEnumerator3"))))))))

(event Custom|CheckEspresso
  (if (>= (Variables|Default|GetAmountEspresso) 1)
    (Variables|Default|SetDrinkType "NewEnumerator1")))

(event EventBeginPlay
  (Utilities|Time|SetTimerbyEvent (delegate Custom|CupFillUpdate) 1.0 true))

(event Collision|EventActorBeginOverlap
  (params (OtherActor :type Actor%20Object%20Reference)))

(event EventTick
  (params (DeltaSeconds :type Float%20%28single-precision%29))
  (bind _liquidfilledindicatormodel_temp (Variables|Default|GetLiquidFilledIndicatorModel_Temp))
  (Utilities|FlowControl|Sequence
    (:then_0
      (Rendering|Components|TextRender|SetText (Variables|Default|GetTypeLabelText) (Utilities|Text|ToText(String) (Utilities|String|EnumtoString (Variables|Default|GetCoffeeType))))
      (Rendering|Components|TextRender|SetText (Variables|Default|GetFillLabelText) (Utilities|Text|ToText(Integer) (Variables|Default|GetCupFilledAmount)))
      (if (>= (Variables|Default|GetAmountEspresso) 1)
        (Variables|Default|SetDrinkType "NewEnumerator1")))
    (:then_1
      (if (>= (Variables|Default|GetAmountEspresso) 1)
        (Rendering|SetVisibility _liquidfilledindicatormodel_temp true false)
        (else
          (Rendering|SetVisibility _liquidfilledindicatormodel_temp false false))))))

(fn ConstructionScript)

(fn FuncCupFillUpdate
  (Utilities|MOnlyifIsCoffee?)
  (Rendering|SetVisibility (Variables|Default|GetLiquidFilledIndicatorModel_Temp) true false)
  (bind _output_get (Variables|Default|SetCupFilledAmount 0))
  (Transformation|SetWorldScale3D (Variables|Default|GetLiquidFilledIndicatorModel_Temp) (Math|Vector|MakeVector 0.0 0.0 (Math|Conversions|ToFloat(Integer) (/ _output_get 100)))))