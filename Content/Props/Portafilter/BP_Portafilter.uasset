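; VR portafilter prop that the player grabs, fills with coffee grounds, uses and empties.
; Events track grounds state and recolor an arrow, while Tick refreshes the grounds mesh and material for tampered or untampered coffee.
; Grab and drop play sounds and set Held and the VR player's OverPorta flag.
; During the tutorial, hovering while not held highlights the mesh and pops up a hint widget with sound, via a DoOnce.
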(event OnDropped(GrabComponent)
  (bind _asvrplayer (Utilities|Casting|CastToVRPlayer (Game|Player|GetPlayerPawn 0)))
  (Variables|/Game/VRTemplate/Blueprints/VRPlayer.VRPlayer_C|SetOverPorta _asvrplayer false)
  (Audio|PlaySoundatLocation "/Game/Audio/dropobject.dropobject" (Transformation|GetActorLocation self) "0, 0, 0" 1.0 1.0 0.0 0 0 0 0)
  (Rendering|SetVisibility (Variables|Default|GetWidget4Hover1) true false)
  (Variables|Default|Setheld false))

(event OnGrabbed(GrabComponent)
  (bind _asvrplayer (Utilities|Casting|CastToVRPlayer (Game|Player|GetPlayerPawn 0)))
  (Variables|/Game/VRTemplate/Blueprints/VRPlayer.VRPlayer_C|SetOverPorta _asvrplayer true)
  (Audio|PlaySoundatLocation "/Game/Audio/pickupobject.pickupobject" (Transformation|GetActorLocation self) "0, 0, 0" 1.0 1.0 0.0 0 0 0 0)
  (Rendering|SetVisibility (Variables|Default|GetWidget4Hover1) false false)
  (Variables|Default|Setheld true))

(event OnComponentBeginOverlap(Sphere)
  (params (OverlappedComponent :type Primitive%20Component%20Object%20Reference) (OtherActor :type Actor%20Object%20Reference) (OtherComp :type Primitive%20Component%20Object%20Reference) (OtherBodyIndex :type Integer) (bFromSweep :type Boolean) (SweepResult :type Hit%20Result%20Structure%20%28by%20ref%29)))

(event Custom|EmptyFilter
  (Variables|Default|SetHasGrounds? false)
  (Variables|Default|SetIsGroundsUsed? false)
  (Rendering|SetVisibility (Variables|Default|GetGroundsIndicatorMesh) false false)
  (Components|Arrow|SetArrowColor(LinearColor) (Variables|Default|GetArrow) "(R=0.000000,G=1.000000,B=0.000000,A=1.000000)")
  (Development|PrintString "Filter Emptied"))

(event Custom|FillFilter
  (Variables|Default|SetHasGrounds? true)
  (Variables|Default|SetIsGroundsUsed? false)
  (Components|Arrow|SetArrowColor(LinearColor) (Variables|Default|GetArrow) "(R=0.091667,G=0.039586,B=0.003474,A=1.000000)")
  (Rendering|SetVisibility (Variables|Default|GetGroundsIndicatorMesh) true false)
  (Development|PrintString "Filter Filled"))

(event Custom|theout
  (bind _staticmesh (Variables|Default|GetStaticMesh))
  (bind _staticmesh_2 (Variables|Default|GetStaticMesh))
  (bind _asvrplayer (Utilities|Casting|CastToVRPlayer (Game|Player|GetPlayerPawn 0)))
  (if (Variables|/Game/VRTemplate/Blueprints/VRPlayer.VRPlayer_C|GetTutorial _asvrplayer)
    (if (Widget|IsHovered (UserInterface|GetWidget (Variables|Default|GetWidget)))
      (if (Variables|Default|Getheld)
        (Rendering|SetVisibility (Variables|Default|GetWidget4Hover1) false false)
        (Rendering|SetRenderCustomDepth _staticmesh false :!label _label)
        (Rendering|Material|SetMaterial _staticmesh_2 0 "/Game/Props/CoffeeFrotherJug/theoc.theoc")
        (CallFunction|Moveuiback)
        (goto _label_2 Reset)
        (else
          (Rendering|SetVisibility (Variables|Default|GetWidget4Hover1) true false)
          (Rendering|SetRenderCustomDepth _staticmesh true)
          (Rendering|Material|SetMaterial _staticmesh_2 0 "/Game/Props/CoffeeFrotherJug/theochover.theochover")
          (Utilities|FlowControl|DoOnce false :!label _label_2
            (:Completed
              (CallFunction|Moveuiup)
              (Audio|PlaySoundatLocation "/Game/dylan_UI/Sounds/maximize_008.maximize_008" (Variables|/Script/Engine.SceneComponent|GetRelativeLocation (Variables|Default|GetStaticMesh)) "0, 0, 0" 1.0 1.0 0.0 0 0 0 0)))))
      (else
        (goto _label)))
    (else
      (Rendering|SetVisibility (Variables|Default|GetWidget4Hover1) false false)
      (goto _label))))

(event Custom|UseGrounds
  (Variables|Default|SetIsGroundsUsed? true)
  (Components|Arrow|SetArrowColor(LinearColor) (Variables|Default|GetArrow) "(R=0.012500,G=0.005993,B=0.002656,A=1.000000)")
  (Development|PrintString "Filter Grounds Used"))

(event Custom|moveuiup
  (bind _widget4hover1 (Variables|Default|GetWidget4Hover1))
  (bind _returnvalue (Transformation|GetRelativeTransform _widget4hover1))
  (Components|MoveComponentTo _widget4hover1 (Math|Vector|MakeVector (.x (.location _returnvalue)) (.y (.location _returnvalue)) (+ (.z (.location _returnvalue)) 1.0)) (.rotation _returnvalue) false false 0.2 false))

(event Custom|moveuiback
  (Transformation|SetRelativeLocation (Variables|Default|GetWidget4Hover1) (Variables|/Script/Engine.SceneComponent|GetRelativeLocation (Variables|Default|GetScene)) false false))

(event EventTick
  (params (DeltaSeconds :type Float%20%28single-precision%29))
  (Utilities|FlowControl|Sequence
    (:then_0
      (CallFunction|IfHasGroundsThenShowGrounds))
    (:then_1
      (CallFunction|Theout))))

(event EventBeginPlay
  (Utilities|FlowControl|Sequence
    (:then_1
      (Variables|Default|Setdefaaultvec (Transformation|GetWorldLocation (Variables|Default|GetWidget4Hover1))))))

(fn ConstructionScript)

(fn IfHasGroundsThenShowGrounds
  (bind _groundsindicatormesh (Variables|Default|GetGroundsIndicatorMesh))
  (if (Variables|Default|GetHasGrounds?)
    (Utilities|FlowControl|Sequence
      (:then_0
        (Rendering|SetVisibility (Variables|Default|GetGroundsIndicatorMesh) true false)
        (bind _asvrplayer (Utilities|Casting|CastToVRPlayer (Game|Player|GetPlayerPawn 0)))
        (Variables|/Game/VRTemplate/Blueprints/VRPlayer.VRPlayer_C|SetOverPorta _asvrplayer false))
      (:then_1
        (if (Variables|Default|GetTampered?)
          (Components|StaticMesh|SetStaticMesh _groundsindicatormesh "/Game/Props/coffeegranules/tamperedcoffee.tamperedcoffee")
          (Rendering|Material|SetMaterial (Variables|Default|GetGroundsIndicatorMesh) 0 "/Game/Props/coffeegranules/tamperedcoffeegranule.tamperedcoffeegranule")
          (else
            (Components|StaticMesh|SetStaticMesh _groundsindicatormesh "/Game/Props/coffeegranules/untamperedcoffee.untamperedcoffee")
            (Rendering|Material|SetMaterial (Variables|Default|GetGroundsIndicatorMesh) 0 "/Game/Props/coffeegranules/coffeegranule.coffeegranule")))))
    (else
      (Rendering|SetVisibility (Variables|Default|GetGroundsIndicatorMesh) false false))))

(fn RemoveGrounds
  (if (Variables|Default|GetHasGrounds?)
    (Variables|Default|SetHasGrounds? false)))