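; VR coffee bag prop that fills an overlapping BP_Portafilter with grounds and plays a sound if it has none.
; A second capsule outlines the bag meshes through custom depth while the VRPlayer overlaps it.
; Fast looping timers poll the player's Tutorial flag to show a hint widget.
; During the tutorial, hovering the hover widget also highlights the bag and raises the hint until hover ends.
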(event OnComponentBeginOverlap(Capsule)
  (params (OverlappedComponent :type Primitive%20Component%20Object%20Reference) (OtherActor :type Actor%20Object%20Reference) (OtherComp :type Primitive%20Component%20Object%20Reference) (OtherBodyIndex :type Integer) (bFromSweep :type Boolean) (SweepResult :type Hit%20Result%20Structure%20%28by%20ref%29))
  (Utilities|FlowControl|Sequence
    (:then_0
      (bind _asbp_portafilter (Utilities|Casting|CastToBP_Portafilter OtherActor))
      (if (not (Variables|/Game/Props/Portafilter/BP_Portafilter.BP_Portafilter_C|GetHasGrounds? _asbp_portafilter))
        (Variables|/Game/Props/Portafilter/BP_Portafilter.BP_Portafilter_C|SetHasGrounds? _asbp_portafilter true)
        (Audio|PlaySoundatLocation "/Game/Audio/coffegrounds/takegrounds.takegrounds" (Transformation|GetActorLocation self) "0, 0, 0" 1.0 1.0 0.0 0 0 0 0)))))

(event OnComponentEndOverlap(Capsule)
  (params (OverlappedComponent :type Primitive%20Component%20Object%20Reference) (OtherActor :type Actor%20Object%20Reference) (OtherComp :type Primitive%20Component%20Object%20Reference) (OtherBodyIndex :type Integer)))

(event OnComponentBeginOverlap(Capsule1UI)
  (params (OverlappedComponent :type Primitive%20Component%20Object%20Reference) (OtherActor :type Actor%20Object%20Reference) (OtherComp :type Primitive%20Component%20Object%20Reference) (OtherBodyIndex :type Integer) (bFromSweep :type Boolean) (SweepResult :type Hit%20Result%20Structure%20%28by%20ref%29))
  (Utilities|Casting|CastToVRPlayer OtherActor)
  (Rendering|SetRenderCustomDepth (Variables|Default|Getcoffeegran) true))

(event OnComponentEndOverlap(Capsule1UI)
  (params (OverlappedComponent :type Primitive%20Component%20Object%20Reference) (OtherActor :type Actor%20Object%20Reference) (OtherComp :type Primitive%20Component%20Object%20Reference) (OtherBodyIndex :type Integer))
  (Utilities|Casting|CastToVRPlayer OtherActor)
  (Rendering|SetRenderCustomDepth (Variables|Default|Getcoffeegran) false))

(event OnComponentBeginOverlap(Widget4Hover)
  (params (OverlappedComponent :type Primitive%20Component%20Object%20Reference) (OtherActor :type Actor%20Object%20Reference) (OtherComp :type Primitive%20Component%20Object%20Reference) (OtherBodyIndex :type Integer) (bFromSweep :type Boolean) (SweepResult :type Hit%20Result%20Structure%20%28by%20ref%29)))

(event Custom|playhovercof
  (bind _asvrplayer (Utilities|Casting|CastToVRPlayer (Game|Player|GetPlayerPawn 0)))
  (if (Variables|/Game/VRTemplate/Blueprints/VRPlayer.VRPlayer_C|GetTutorial _asvrplayer)
    (if (Widget|IsHovered (UserInterface|GetWidget (Variables|Default|GetWidget4Hover)))
      (Rendering|SetRenderCustomDepth (Variables|Default|Getcoffeegran) true)
      (Utilities|FlowControl|DoOnce false :!label _label
        (:Completed
          (CallFunction|Changeloc)))
      (else
        (Rendering|SetRenderCustomDepth (Variables|Default|Getcoffeegran) false)
        (CallFunction|Changebackloc)
        (goto _label Reset)))))

(event Custom|changeloc
  (bind _widget4hover1 (Variables|Default|GetWidget4Hover1))
  (bind _returnvalue (Transformation|GetWorldLocation _widget4hover1))
  (Transformation|SetWorldLocation _widget4hover1 (Math|Vector|MakeVector (.x _returnvalue) (.y _returnvalue) (+ (.z _returnvalue) 15.0)) false false))

(event Custom|changebackloc
  (Transformation|SetWorldLocation (Variables|Default|GetWidget4Hover1) (Variables|Default|Gethoverloc) false false))

(event Custom|tutorialactive
  (bind _asvrplayer (Utilities|Casting|CastToVRPlayer (Game|Player|GetPlayerPawn 0)))
  (if (Variables|/Game/VRTemplate/Blueprints/VRPlayer.VRPlayer_C|GetTutorial _asvrplayer)
    (Rendering|SetVisibility (Variables|Default|GetWidget4Hover1) true false)
    (else
      (Rendering|SetVisibility (Variables|Default|GetWidget4Hover1) false false))))

(event EventBeginPlay
  (Utilities|FlowControl|Sequence
    (:then_0
      (Utilities|Time|SetTimerbyEvent (delegate Custom|playhovercof) 0.01 true))
    (:then_1
      (Variables|Default|Sethoverloc (Transformation|GetWorldLocation (Variables|Default|GetWidget4Hover1))))
    (:then_2
      (Utilities|Time|SetTimerbyEvent (delegate Custom|tutorialactive) 0.01 true))))

(event Collision|EventActorBeginOverlap
  (params (OtherActor :type Actor%20Object%20Reference)))

(event EventTick
  (params (DeltaSeconds :type Float%20%28single-precision%29)))

(event EventInteract)

(fn ConstructionScript)