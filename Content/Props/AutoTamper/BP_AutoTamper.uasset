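; BP_AutoTamper is a VR lever-operated coffee tamper prop.
; Grabbing the lever hides the player's hands, enables tamping and plays a lever sequence, which reverses on drop; sequencer events also toggle tamping.
; While enabled, a trigger box marks overlapping portafilters with untamped grounds as tamped and plays a sound.
; A second box highlights the lever for nearby players via custom depth and material swaps.
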(event OnGrabbed(GrabComponent)
  (Variables|Default|Setcantamper true)
  (bind _asvrplayer (Utilities|Casting|CastToVRPlayer (Game|Player|GetPlayerPawn 0)))
  (Variables|/Game/VRTemplate/Blueprints/VRPlayer.VRPlayer_C|SetPlayerHideHands _asvrplayer true)
  (Default|Hidehands _asvrplayer)
  (Sequencer|Player|Play (Variables|/Script/ActorSequence.ActorSequenceComponent|GetSequencePlayer (Variables|Default|Getleverdown)) :!class /Script/MovieScene.MovieSceneSequencePlayer))

(event OnDropped(GrabComponent)
  (Variables|Default|Setcantamper false)
  (bind _asvrplayer (Utilities|Casting|CastToVRPlayer (Game|Player|GetPlayerPawn 0)))
  (Variables|/Game/VRTemplate/Blueprints/VRPlayer.VRPlayer_C|SetPlayerHideHands _asvrplayer false)
  (Default|Hidehands _asvrplayer)
  (Class|MovieSceneSequencePlayer|PlayReverse (Variables|/Script/ActorSequence.ActorSequenceComponent|GetSequencePlayer (Variables|Default|Getleverdown))))

(event OnComponentBeginOverlap(Box)
  (params (OverlappedComponent :type Primitive%20Component%20Object%20Reference) (OtherActor :type Actor%20Object%20Reference) (OtherComp :type Primitive%20Component%20Object%20Reference) (OtherBodyIndex :type Integer) (bFromSweep :type Boolean) (SweepResult :type Hit%20Result%20Structure%20%28by%20ref%29))
  (if (Variables|Default|Getcantamper)
    (bind _asbp_portafilter (Utilities|Casting|CastToBP_Portafilter OtherActor))
    (if (and (!= (Variables|/Game/Props/Portafilter/BP_Portafilter.BP_Portafilter_C|GetTampered? _asbp_portafilter) true) (== (Variables|/Game/Props/Portafilter/BP_Portafilter.BP_Portafilter_C|GetHasGrounds? _asbp_portafilter) true))
      (Variables|/Game/Props/Portafilter/BP_Portafilter.BP_Portafilter_C|SetTampered? _asbp_portafilter true)
      (Audio|PlaySoundatLocation 0 (Transformation|GetWorldLocation (Variables|/Game/Props/Portafilter/BP_Portafilter.BP_Portafilter_C|GetSphere _asbp_portafilter)) "0, 0, 0" 1.0 1.0 0.0 0 0 0 0))))

(event OnComponentBeginOverlap(Box1)
  (params (OverlappedComponent :type Primitive%20Component%20Object%20Reference) (OtherActor :type Actor%20Object%20Reference) (OtherComp :type Primitive%20Component%20Object%20Reference) (OtherBodyIndex :type Integer) (bFromSweep :type Boolean) (SweepResult :type Hit%20Result%20Structure%20%28by%20ref%29))
  (bind _leveraction (Variables|Default|Getleveraction))
  (Utilities|Casting|CastToVRPlayer OtherActor)
  (Rendering|SetRenderCustomDepth _leveraction true)
  (Rendering|Material|SetMaterial _leveraction 0 "/Game/Props/CoffeeFrotherJug/theochover.theochover"))

(event OnComponentEndOverlap(Box1)
  (params (OverlappedComponent :type Primitive%20Component%20Object%20Reference) (OtherActor :type Actor%20Object%20Reference) (OtherComp :type Primitive%20Component%20Object%20Reference) (OtherBodyIndex :type Integer))
  (bind _leveraction (Variables|Default|Getleveraction))
  (Utilities|Casting|CastToVRPlayer OtherActor)
  (Rendering|SetRenderCustomDepth _leveraction false)
  (Rendering|Material|SetMaterial _leveraction 0 "/Game/Props/AutoTamper/the_coffeema.the_coffeema"))

(event Custom|dfsdf
  (if true
    _))

(event Custom|CustomEvent_0
  (Transformation|AttachComponentToComponent (Variables|Default|GetmlkjugUI) (Variables|Default|Getpress) "None" "KeepRelative" "KeepRelative" "KeepRelative" true))

(event EventBeginPlay)

(event Collision|EventActorBeginOverlap
  (params (OtherActor :type Actor%20Object%20Reference)))

(event EventTick
  (params (DeltaSeconds :type Float%20%28single-precision%29))
  (CallFunction|CustomEvent0))

(event Custom|disabletamp
  (params (Owner :type Actor%20Object%20Reference))
  (Variables|Default|Setcantamper false))

(event Custom|enabletmap
  (params (Owner :type Actor%20Object%20Reference))
  (Variables|Default|Setcantamper true))

(fn ConstructionScript)